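; Breakout-style ball actor that launches its physics sphere on BeginPlay and caches the player's paddle pawn.
; Each hit raises BallSpeed and clamps velocity to exactly that speed, updating the score through the paddle's HUD for Brick-tagged actors.
; On destruction it asks the spawner for a new ball while the paddle has lives left, otherwise shows the Game Over widget.
; The E key destroys every brick in the level.
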(event `self.ReceiveBeginPlay`
  (`PrimitiveComponent.AddImpulse` (`self.Sphere`) (0.0 600.0 0.0) "None" true)
  (bind _aspaddle_blueprint (cast `/Game/Blueprint/Paddle_blueprint` (`GameplayStatics.GetPlayerPawn` 0)))
  (set `self.As Paddle Blueprint` _aspaddle_blueprint))

(event `Key|E`
  (params (Key :type "Key Structure"))
  (:`Pressed`
    (bind _outactors (`GameplayStatics.GetAllActorsOfClass` "/Game/Blueprint/Brick_BP.Brick_BP_C"))
    (for _array_element _outactors
      (`self.K2_DestroyActor` _array_element))))

(event `self.ReceiveHit`
  (params (MyComp :type "PrimitiveComponent Object Reference") (Other :type "Actor Object Reference") (OtherComp :type "PrimitiveComponent Object Reference") (bSelfMoved :type Boolean) (HitLocation :type "Vector Structure") (HitNormal :type "Vector Structure") (NormalImpulse :type "Vector Structure") (Hit :type "HitResult Structure (by ref)"))
  (bind _sphere (`self.Sphere`))
  (bind _ball_speed (`self.Ball_speed`))
  (set `self.Ball_speed` (+ (`self.Ball_speed`) 15.0))
  (bind _returnvalue (`PrimitiveComponent.GetPhysicsLinearVelocity` _sphere "None"))
  (`PrimitiveComponent.SetPhysicsLinearVelocity` _sphere (`KismetMathLibrary.ClampVectorSize` _returnvalue _ball_speed _ball_speed) false "None")
  (if (`self.ActorHasTag` Other "Brick")
    (`/Game/Blueprint/Player_HUD_WB.Update Score` (`/Game/Blueprint/Paddle_blueprint.PLayer_HUD` (`self.As Paddle Blueprint`)))))

(event `self.ReceiveDestroyed`
  (if (> (`/Game/Blueprint/Paddle_blueprint.Lives` (`self.As Paddle Blueprint`)) 0)
    (`/Game/Blueprint/Ball_Spawner_BP.Spawn Ball` (`self.Ball_Spawner_REF`))
    (else
      (bind _returnvalue (`|CreateWidget` "/Game/Blueprint/Game_Over_WB.Game_Over_WB_C"))
      (`UserWidget.AddToViewport` _returnvalue 0))))

(fn `UserConstructionScript`)