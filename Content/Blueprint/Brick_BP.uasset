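; Destructible brick for a Breakout-style game, with a strength value that sets its glowing material color.
; Each Ball_BP hit decrements strength and recolors the brick, or at zero spawns an explosion and destroys it.
; When no bricks remain, the level number from Level_tracker_BP selects the next level to open, or the win widget after level seven.
; The construction script applies the color from the initial strength.
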(event `self.ReceiveHit`
  (params (MyComp :type "PrimitiveComponent Object Reference") (Other :type "Actor Object Reference") (OtherComp :type "PrimitiveComponent Object Reference") (bSelfMoved :type Boolean) (HitLocation :type "Vector Structure") (HitNormal :type "Vector Structure") (NormalImpulse :type "Vector Structure") (Hit :type "HitResult Structure (by ref)"))
  (cast `/Game/Blueprint/Ball_BP` Other)
  (bind _result (`/Engine/EditorBlueprintResources/StandardMacros.DecrementInt` (`self.Brick_Strength`))
    (:`  `
      (if (== _result 0)
        (`GameplayStatics.SpawnEmitterAtLocation` "/Game/StarterContent/Particles/P_Explosion.P_Explosion" (`self.K2_GetActorLocation`))
        (`self.K2_DestroyActor`)
        (bind _outactors (`GameplayStatics.GetAllActorsOfClass` "Brick_BP_C"))
        (if (== (`KismetArrayLibrary.Array_Length` _outactors) 0)
          (bind _returnvalue (`GameplayStatics.GetActorOfClass` "/Game/Blueprint/Level_tracker_BP.Level_tracker_BP_C"))
          (switch `int` (`/Game/Blueprint/Level_tracker_BP.LEVELNUMBER` _returnvalue)
            (:`1`
              (`GameplayStatics.OpenLevelBySoftObjectPtr` "/Game/maps/level2.level2"))
            (:`2`
              (`GameplayStatics.OpenLevelBySoftObjectPtr` "/Game/maps/level3.level3"))
            (:`3`
              (`GameplayStatics.OpenLevelBySoftObjectPtr` "/Game/maps/level4.level4"))
            (:`4`
              (`GameplayStatics.OpenLevelBySoftObjectPtr` "/Game/maps/level5.level5"))
            (:`5`
              (`GameplayStatics.OpenLevelBySoftObjectPtr` "/Game/maps/level6.level6"))
            (:`6`
              (`GameplayStatics.OpenLevelBySoftObjectPtr` "/Game/maps/level7.level7"))
            (:`7`
              (bind _returnvalue_2 (`|CreateWidget` "/Game/Blueprint/Win_WB.Win_WB_C"))
              (`UserWidget.AddToViewport` _returnvalue_2 0))))
        (else
          (`self.Update_Brick_Color`))))))

(fn `Update_Brick_Color`
  (bind _cube (`self.Cube`))
  (switch `int` (`self.Brick_Strength`)
    (:`1`
      (`PrimitiveComponent.SetMaterial` _cube 0 "/Game/Materials/Yellow_glowing_Mat.Yellow_glowing_Mat"))
    (:`2`
      (`PrimitiveComponent.SetMaterial` _cube 0 "/Game/Materials/Red_Glowing_Mat.Red_Glowing_Mat"))
    (:`3`
      (`PrimitiveComponent.SetMaterial` _cube 0 "/Game/Materials/Green_glowing_Mat.Green_glowing_Mat"))))

(fn `UserConstructionScript`
  (`self.Update_Brick_Color`))